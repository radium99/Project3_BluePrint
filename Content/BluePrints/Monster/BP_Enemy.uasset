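; Enemy monster Blueprint that runs a Locomotion, Chase, Attack and Dead state machine, mirrored to the AI Blackboard.
; AI perception stores a sensed player as target and can start a chase, which ends beyond a fixed distance.
; UpdateState sets movement speed from level-based enemy data, stops movement for Attack and Dead, and locks once dead.
; Damage goes to the HP controller; other per-state handlers are empty stubs.
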(event `self.ReceiveTick`
  (params (DeltaSeconds :type "Float (single-precision)"))
  (switch `/Game/BluePrints/Monster/EEnemyState` (`self.State_BP`)
    (:`NewEnumerator0`
      (`self.OnLocomotion`))
    (:`NewEnumerator1`
      (`self.OnChase`))
    (:`NewEnumerator2`
      (`self.OnAttack`))
    (:`NewEnumerator3`
      (`self.OnDead`))))

(event `self.ReceiveAnyDamage`
  (params (Damage :type "Float (single-precision)") (DamageType :type "DamageType Object Reference") (InstigatedBy :type "Controller Object Reference") (DamageCauser :type "Actor Object Reference"))
  (`/Game/BluePrints/Componants/BP_HPController.RecieveDamage` (`self.BP_HPController`) Damage))

(event `self.AIPerception.OnTargetPerceptionUpdated`
  (params (Actor :type "Actor Object Reference") (Stimulus :type "AIStimulus Structure"))
  (if (`.bSuccessfullySensed` (break `AIStimulus` Stimulus))
    (if (`|EnumEquality` (`self.State_BP`) "NewEnumerator0")
      (if (`self.ActorHasTag` Actor "Player")
        (`BlackboardComponent.SetValueAsObject` (`AIController.Blackboard` (`AIBlueprintHelperLibrary.GetAIController` self)) (`self.Target Key`) Actor)
        (bind _asbp_character (cast `/Game/BluePrints/Character/BP_Character` Actor))
        (if (`|EnumInequality` (`/Game/BluePrints/Character/BP_Character.State_BP` _asbp_character) "NewEnumerator2")
          (`self.Update State` "NewEnumerator1"))))))

(event `Update State`
  (params (`New State` :type "/Game/BluePrints/Monster/EEnemyState Enum" :default "NewEnumerator0"))
  (bind _charactermovement (`self.CharacterMovement`))
  (bind (_current_leveldata_attack _current_leveldata_defence _current_leveldata_walkspeed _current_leveldata_chasespeed) (break `/Game/BluePrints/Monster/Data/BP_EnemyLevelData` (`/Game/BluePrints/Monster/Data/BP_EnemyData.GetCurrentLevelData` (`self.BP_EnemyData`))))
  ; 상태 변경
  (if (`|EnumInequality` (`self.State_BP`) "NewEnumerator3")
    (bind _output_get (set `self.State_BP` `New State`))
    (`BlackboardComponent.SetValueAsEnum` (`AIController.Blackboard` (`AIBlueprintHelperLibrary.GetAIController` self)) (`self.State Key`) _output_get)
    (switch `/Game/BluePrints/Monster/EEnemyState` (`self.State_BP`)
      (:`NewEnumerator0`
        (set `CharacterMovementComponent.MaxWalkSpeed` _current_leveldata_walkspeed _charactermovement))
      (:`NewEnumerator1`
        (set `CharacterMovementComponent.MaxWalkSpeed` _current_leveldata_chasespeed _charactermovement))
      (:`NewEnumerator2`
        (set `CharacterMovementComponent.MaxWalkSpeed` 0.0 _charactermovement :!label _label))
      (:`NewEnumerator3`
        (goto _label)))))

(fn `OnAttack`)

(fn `OnChase`
  (bind _asactor (cast `Actor` (`BlackboardComponent.GetValueAsObject` (`AIController.Blackboard` (`AIBlueprintHelperLibrary.GetAIController` self)) (`self.Target Key`))))
  (if (> (`KismetMathLibrary.Vector_Distance` (`self.K2_GetActorLocation` _asactor) (`self.K2_GetActorLocation`)) 700.0)
    (`self.Update State` "NewEnumerator0")))

(fn `OnDead`)

(fn `OnLocomotion`)

(fn `TurnToTarget`)

(fn `UserConstructionScript`)