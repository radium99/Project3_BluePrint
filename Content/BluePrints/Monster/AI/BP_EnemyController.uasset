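; BP_EnemyController is the AI controller for enemy monsters, starting their behavior tree when it possesses a pawn.
; On possess it sets up the BB_Enemy blackboard and runs BT_Enemy.
; It then seeds the blackboard with the pawn's spawn location as home, a default patrol wait time and the initial state.
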(event `self.ReceivePossess`
  (params (PossessedPawn :type "Pawn Object Reference"))
  (`|ExecutionSequence`
    (:`then_0`
      (`self.UseBlackboard` "/Game/BluePrints/Monster/AI/BB_Enemy.BB_Enemy"))
    (:`then_1`
      (`self.RunBehaviorTree` "/Game/BluePrints/Monster/AI/BT_Enemy.BT_Enemy"))
    (:`then_2`
      (`BlackboardComponent.SetValueAsVector` (`AIBlueprintHelperLibrary.GetBlackboard` null) (`self.HomeLocationKey`) (`self.K2_GetActorLocation` PossessedPawn))
      (`BlackboardComponent.SetValueAsFloat` (`AIBlueprintHelperLibrary.GetBlackboard` null) (`self.PatrolWaitTimeKey`) 3.0)
      (`BlackboardComponent.SetValueAsEnum` (`AIBlueprintHelperLibrary.GetBlackboard` null) (`self.StateKey`) 0))))

(fn `UserConstructionScript`)