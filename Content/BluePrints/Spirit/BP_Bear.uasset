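; Bear spirit AI character that follows the player, driven by a Follow/Chase/Attack/Dead state.
; Sight perception stores the player as the Blackboard target and re-enters Follow if the player is alive.
; UpdateState mirrors state to the Blackboard and sets walk speed from level-based spirit data, locking once Dead.
; Tick dispatches per-state handlers, but only OnFollow has logic, re-applying Follow; Chase and Dead handlers are empty.
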(event `self.ReceiveBeginPlay`)

(event `self.ReceiveTick`
  (params (DeltaSeconds :type "Float (single-precision)"))
  ; 간단한 이동 처리(플레이어를 따라다님)
  (switch `/Game/BluePrints/Spirit/ESpiritState` (`self.State_BP`)
    (:`NewEnumerator0`
      (`self.OnFollow`))
    (:`NewEnumerator1`
      (`self.OnChase`))
    (:`NewEnumerator3`
      (`self.OnDead`))))

(event `FollowPlayer`
  ; 간단한 이동 처리(플레이어를 따라다님)
  (`|AIMoveTo` self (0.0 0.0 0.0) (`GameplayStatics.GetPlayerCharacter` 0) 0.0
    (:`OnSuccess`
      (`self.FollowPlayer`))))

(event `self.AIPerception.OnTargetPerceptionUpdated`
  (params (Actor :type "Actor Object Reference") (Stimulus :type "AIStimulus Structure"))
  ; 시야 감지
  (if (`.bSuccessfullySensed` (break `AIStimulus` Stimulus))
    (if (`|EnumEquality` (`self.State_BP`) "NewEnumerator0")
      (if (`self.ActorHasTag` Actor "Player")
        (`BlackboardComponent.SetValueAsObject` (`AIController.Blackboard` (`AIBlueprintHelperLibrary.GetAIController` self)) (`self.Target Player Key`) Actor)
        ;; 플레이어가 죽었는지 확인
        (bind _asbp_character (cast `/Game/BluePrints/Character/BP_Character` Actor))
        (if (not (`|EnumEquality` (`/Game/BluePrints/Character/BP_Character.State_BP` _asbp_character) "NewEnumerator2"))
          (`self.UpdateState` "NewEnumerator0"))))))

(event `UpdateState`
  (params (`New State` :type "/Game/BluePrints/Spirit/ESpiritState Enum" :default "NewEnumerator0"))
  (bind _charactermovement (`self.CharacterMovement`))
  (bind (_current_leveldata_attack _current_leveldata_defence _current_leveldata_walkspeed _current_leveldata_chasespeed) (break `/Game/BluePrints/Spirit/Data/BP_SpiritLevelData` (`/Game/BluePrints/Spirit/Data/BP_SpiritData.GetCurrentLevelData` (`self.BP_SpiritData`))))
  ; 몬스터 상태 변경 이벤트
  (if (`|EnumInequality` (`self.State_BP`) "NewEnumerator3")
    (bind _output_get (set `self.State_BP` `New State`))
    (`BlackboardComponent.SetValueAsEnum` (`AIController.Blackboard` (`AIBlueprintHelperLibrary.GetAIController` self)) (`self.State Key`) _output_get)
    (switch `/Game/BluePrints/Spirit/ESpiritState` (`self.State_BP`)
      (:`NewEnumerator0`
        (set `CharacterMovementComponent.MaxWalkSpeed` _current_leveldata_walkspeed _charactermovement))
      (:`NewEnumerator1`
        (set `CharacterMovementComponent.MaxWalkSpeed` _current_leveldata_chasespeed _charactermovement))
      (:`NewEnumerator2`
        (set `CharacterMovementComponent.MaxWalkSpeed` 0.0 _charactermovement :!label _label))
      (:`NewEnumerator3`
        (goto _label)))))

(fn `OnChase`)

(fn `OnDead`)

(fn `OnFollow`
  (bind _asactor (cast `Actor` (`BlackboardComponent.GetValueAsObject` (`AIController.Blackboard` (`AIBlueprintHelperLibrary.GetAIController` self)) (`self.Target Player Key`))))
  (if (> (`KismetMathLibrary.Vector_Distance` (`self.K2_GetActorLocation` _asactor) (`self.K2_GetActorLocation`)) 0.0)
    (`self.UpdateState` "NewEnumerator0")))

(fn `TurnToTarget`
  (params (TargetPlayer :type "Actor Object Reference"))
  (switch `/Game/BluePrints/Spirit/ESpiritState` (`self.State_BP`)
    (:`NewEnumerator0`
      (`self.K2_SetActorRotation` (`KismetMathLibrary.MakeRotFromX` (- (`self.K2_GetActorLocation` TargetPlayer) (`self.K2_GetActorLocation`)))))))

(fn `UserConstructionScript`)