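; AI controller for the spirit, which starts its behavior tree and seeds its blackboard when it possesses a pawn.
; On possess it sets up BB_Spirit, runs BT_Spirit, then stores the pawn's location as the home reference point and sets the state to the default Follow.
; A node that would set the patrol wait time is present but never runs.
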(event `self.ReceivePossess`
  (params (PossessedPawn :type "Pawn Object Reference"))
  (`|ExecutionSequence`
    (:`then_0`
      (`self.UseBlackboard` "/Game/BluePrints/Spirit/AI/BB_Spirit.BB_Spirit"))
    (:`then_1`
      (`self.RunBehaviorTree` "/Game/BluePrints/Spirit/AI/BT_Spirit.BT_Spirit"))
    (:`then_2`
      ; 멀어지거나 다시 돌아가기 위한 기준점
      (`BlackboardComponent.SetValueAsVector` (`AIBlueprintHelperLibrary.GetBlackboard` null) (`self.HomeLocationKey`) (`self.K2_GetActorLocation` PossessedPawn)) ; 블랙보드 데이터 갱신
      ; 시작할 때 BlackBoard의 상태값 동기화
      (`BlackboardComponent.SetValueAsEnum` (`AIBlueprintHelperLibrary.GetBlackboard` null) (`self.StateKey`) 0) ; spawn없으니까 기본은 Follow(0)로 설정
    )))

(fn `UserConstructionScript`)