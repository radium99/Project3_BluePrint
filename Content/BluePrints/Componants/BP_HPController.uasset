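; Health component that tracks an actor's current and maximum hit points and signals damage and death.
; Health starts at the maximum on BeginPlay, and UpdateNextHp sets a new maximum and refills to it.
; RecieveDamage subtracts damage only while health is above zero, clamps it at zero, fires the dead event, and broadcasts the HP-changed event with current and maximum values.
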(event `self.ReceiveBeginPlay`
  ; 시작할 때 최대 체력으로 설정
  (set `self.HealthPoint` (`self.MaxHealthPoint`)))

(event `RecieveDamage`
  (params (Damage :type "Float (double-precision)"))
  ; 대미지 처리 - 과정에서 죽음 이벤트 발생
  (if (> (`self.HealthPoint`) 0.0)
    (bind _output_get (set `self.HealthPoint` (- (`self.HealthPoint`) Damage)))
    (if (<= _output_get 0.0)
      (set `self.HealthPoint` 0.0)
      (`self.DeadEvent`)
      (`self.OnHpChanged` (`self.HealthPoint`) (`self.MaxHealthPoint`))
      (else
        (`self.OnHpChanged` (`self.HealthPoint`) (`self.MaxHealthPoint`))))))

(event `UpdateNextHp`
  (params (`Max Health Point` :type "Float (double-precision)"))
  (bind _output_get (set `self.MaxHealthPoint` `Max Health Point`))
  (set `self.HealthPoint` _output_get))